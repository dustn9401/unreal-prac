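; Rifle fire ability that handles the cosmetic and impact response once the shot's target data is ready.
; It executes the ranged weapon fire GameplayCue from the first hit result.
; For hits with a valid physical material, it feeds position, normal and surface type to lazily spawned, reused decal and impact actors, passing the muzzle socket position to the latter.
; It then detonates any hit UPFExplosive.
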(event Ability|EventActivateAbility)

(event Ability|EventOnEndAbility
  (params (bWasCancelled :type Boolean)))

(event EventOnTargetDataReady
  (params (InData :type Gameplay%20Ability%20Target%20Data%20Handle%20Structure%20%28by%20ref%29))
  (bind _returnvalue (Ability|TargetData|GetHitResultfromTargetData InData))
  (bind _output_get (Variables|Default|SetGCNParam (GameplayCue|MakeGameplayCueParametersfromHitResult (Ability|TargetData|GetHitResultfromTargetData InData))))
  (Class|GameplayAbility|ExecuteGameplayCuewithParams "(TagName=\"GameplayCue.RangedWeapon.Fire\")" _output_get)
  (Variables|Default|SetReturn%20Value%20Hit%20Actor (.hitactor _returnvalue))
  (Variables|Default|SetImpactPositions (Utilities|Array|MakeArray (.location _returnvalue)))
  (Variables|Default|SetImpactNormals (Utilities|Array|MakeArray (.normal _returnvalue)))
  (bind _output_get_2 (Variables|Default|SetReturn%20Value%20Phys%20Mat (.physmat _returnvalue)))
  (Utilities|IsValid _output_get_2
    (:Is%20Valid
      (Variables|Default|SetImpactSurfaces (Utilities|Array|MakeArray (Math|Conversions|ToInteger(Byte) (Variables|/Script/PhysicsCore.PhysicalMaterial|GetSurfaceType _output_get_2))))
      ;[1 1 1] Create Decal Actor If Null
      (Utilities|IsValid (Variables|Default|GetWeaponDecalInstance)
        (:Is%20Valid
          _)
        (:Is%20Not%20Valid
          (bind _returnvalue_2 (Game|SpawnActorfromClass "/Game/UnrealPortfolio/Blueprints/BP_WeaponDecal.BP_WeaponDecal_C" (Math|Transform|MakeTransform "0, 0, 0") "Undefined" "MultiplyWithRoot" 0 0))
          (Variables|Default|SetWeaponDecalInstance _returnvalue_2)))
      (Default|SetData (Variables|Default|GetWeaponDecalInstance) (Variables|Default|GetImpactPositions) (Variables|Default|GetImpactNormals) (Variables|Default|GetImpactSurfaces))
      ;[1 1 1] Create Impact Actor If Null
      (Utilities|IsValid (Variables|Default|GetWeaponImpactInstance)
        (:Is%20Valid
          _)
        (:Is%20Not%20Valid
          (bind _returnvalue_3 (Game|SpawnActorfromClass "/Game/UnrealPortfolio/Blueprints/BP_WeaponImpact.BP_WeaponImpact_C" (Math|Transform|MakeTransform "0, 0, 0") "Undefined" "MultiplyWithRoot" 0 0))
          (Variables|Default|SetWeaponImpactInstance _returnvalue_3)))
      (Default|SetData (Variables|Default|GetWeaponImpactInstance) (Variables|Default|GetImpactPositions) (Variables|Default|GetImpactNormals) (Variables|Default|GetImpactSurfaces) (Transformation|GetSocketLocation (Variables|/Script/UnrealPortfolio.UPFItemInstanceBase|GetMeshComp (Class|UPFGameplayAbilityRangedWeapon|GetWeaponInstance)) "b_gun_muzzleflashSocket"))
      (bind _asupfexplosive (Utilities|Casting|CastToUPFExplosive (Variables|Default|GetReturn%20Value%20Hit%20Actor)))
      (Class|UPFExplosive|Explode _asupfexplosive))))