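; Ranged weapon Blueprint that plays muzzle flash and fire sound when OnFire is called.
; It lazily spawns a rifle Niagara effect at the muzzle socket, reuses it by resetting once finished, toggles its trigger parameter, and aims it at the target data's first hit location.
; It likewise creates one attached audio component and reuses it by sending a "Fire" trigger parameter for each shot.
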(event Custom|OnParticlaFinished
  (params (PSystem :type Niagara%20Component%20Object%20Reference))
  ;[1 1 1] 총구 이펙트
  (Variables|Default|SetIsParticleFinished true))

(event EventBeginPlay)

(event Collision|EventActorBeginOverlap
  (params (OtherActor :type Actor%20Object%20Reference)))

(event EventTick
  (params (DeltaSeconds :type Float%20%28single-precision%29)))

(event EventOnFire
  (params (InData :type Gameplay%20Ability%20Target%20Data%20Handle%20Structure%20%28by%20ref%29))
  (bind _meshcomp (Variables|Default|GetMeshComp))
  (Variables|Default|SetIn%20Data InData)
  (Utilities|FlowControl|Sequence
    (:then_0
      ;[1 1 1] 총구 이펙트
      (Utilities|IsValid (Variables|Default|GetPS_MuzzleFlash)
        (:Is%20Valid
          (if (Variables|Default|GetIsParticleFinished)
            (Niagara|ResetSystem (Variables|Default|GetPS_MuzzleFlash))
            (Variables|Default|SetIsParticleFinished false)))
        (:Is%20Not%20Valid
          (bind _returnvalue (Niagara|SpawnSystemAttached "/Game/Effects/Particles/Weapons/NS_WeaponFire_MuzzleFlash_Rifle.NS_WeaponFire_MuzzleFlash_Rifle" _meshcomp "None" (.location (Transformation|GetSocketTransform _meshcomp (Variables|Default|GetMuzzleSocketName) "RTS_Actor")) "0.000000,90.000000,0.000000" "KeepRelativeOffset" false))
          (Variables|Default|SetPS_MuzzleFlash _returnvalue)
          (Variables|Default|SetMuzzleFlashTrigger false)))
      (bind _output_get (Variables|Default|SetMuzzleFlashTrigger (not (Variables|Default|GetMuzzleFlashTrigger))))
      (Class|NiagaraComponent|SetVariableBool (Variables|Default|GetPS_MuzzleFlash) "User.Trigger" _output_get)
      (EventDispatchers|BindEventtoOnSystemFinished (Variables|Default|GetPS_MuzzleFlash) (delegate Custom|OnParticlaFinished))
      (Niagara|SetNiagaraVariable(Vector3) (Variables|Default|GetPS_MuzzleFlash) "User.Direction" (Math|Vector|Normalize (- (.location (Ability|TargetData|GetHitResultfromTargetData (Variables|Default|GetIn%20Data))) (.Location (Math|Transform|BreakTransform (Transformation|GetSocketTransform (Variables|Default|GetMeshComp) (Variables|Default|GetMuzzleSocketName) "RTS_World")))))))
    (:then_1
      ;[1 1 1] 총구 사운드
      (Utilities|IsValid (Variables|Default|GetAudio%20Component)
        (:Is%20Valid
          _)
        (:Is%20Not%20Valid
          (bind _returnvalue_2 (Audio|SpawnSoundAttached "/Game/Audio/Sounds/Weapons/Rifle2/MSS_Weapons_Rifle2_Fire.MSS_Weapons_Rifle2_Fire" (Variables|Default|GetMeshComp) (Variables|Default|GetMuzzleSocketName) "0, 0, 0" "0, 0, 0" "KeepRelativeOffset" false 1.0 1.0 0.0 0 0))
          (Variables|Default|SetAudio%20Component _returnvalue_2)
          (Utilities|IsValid (Variables|Default|GetAudio%20Component)
            (:Is%20Valid
              _))))
      (Class|AudioParameterControllerInterface|SetTriggerParameter (Variables|Default|GetAudio%20Component) "Fire"))))

(fn ConstructionScript)