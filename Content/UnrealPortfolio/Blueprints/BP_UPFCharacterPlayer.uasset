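; BP_UPFCharacterPlayer is the player character Blueprint, adding death timing, aim-down-sights camera motion and a slow-motion key.
; When death starts, it waits briefly before calling FinishDeath.
; The TL_ADS timeline plays or reverses, scaling the camera boom arm length from the TargetArmLength in CharacterControlData.
; Holding F lowers global time dilation, and releasing it restores normal speed.
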(event Custom|Reverse%20TL_ADS
  (bind _armlength (Timeline|TL_ADS Reverse)
    (:Update
      (Variables|/Script/Engine.SpringArmComponent|SetTargetArmLength (Variables|Default|GetCameraBoom) (* _armlength (Variables|/Script/UnrealPortfolio.UPFCharacterControlData|GetTargetArmLength (Variables|Default|GetCharacterControlData)))))))

(event Custom|Play%20TL_ADS
  (bind _armlength (Timeline|TL_ADS Play)
    (:Update
      (Variables|/Script/Engine.SpringArmComponent|SetTargetArmLength (Variables|Default|GetCameraBoom) (* _armlength (Variables|/Script/UnrealPortfolio.UPFCharacterControlData|GetTargetArmLength (Variables|Default|GetCharacterControlData)))))))

(event EventBeginPlay)

(event Collision|EventActorBeginOverlap
  (params (OtherActor :type Actor%20Object%20Reference)))

(event EventTick
  (params (DeltaSeconds :type Float%20%28single-precision%29)))

(event EventOnDeathStart
  (Utilities|FlowControl|Delay 5.0)
  (Class|UPFCharacterBase|FinishDeath))

(event Input|KeyboardEvents|F
  (params (Key :type Key%20Structure :default "None"))
  (:Pressed
    (Utilities|Time|SetGlobalTimeDilation 0.2))
  (:Released
    (Utilities|Time|SetGlobalTimeDilation 1.0)))

(fn ConstructionScript
  (|CallParentFunction))