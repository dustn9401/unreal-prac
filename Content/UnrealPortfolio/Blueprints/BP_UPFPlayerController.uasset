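; Player controller that owns the local player's HUD and game result popup.
; On BeginPlay it sets game-only input and adds the HUD widget for the local controller.
; Game over shows a Fail result widget locally, switching to UI-only input with cursor, while non-local controllers just print a death message.
; Closing the popup restores game input, then respawns or quits based on the returned result.
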(event Custom|ShowGameResultWidget
  (params (GameResult :type Gameplay%20Tag%20Structure))
  (bind _returnvalue (UserInterface|CreateWidget "/Game/UnrealPortfolio/UI/WBP_GameResult.WBP_GameResult_C" self))
  (Utilities|FlowControl|Sequence
    (:then_0
      (Input|SetInputModeUIOnly self _returnvalue "DoNotLock" false)
      (Variables|Default|SetbShowMouseCursor true))
    (:then_1
      (UserInterface|Viewport|AddtoViewport _returnvalue 0))
    (:then_2
      (Default|SetData _returnvalue GameResult))))

(event Custom|CloseGameResultWidget
  (params (PopupResult :type Name))
  (Variables|Default|SetPopup%20Result PopupResult)
  (Utilities|FlowControl|Sequence
    (:then_0
      (Input|SetInputModeGameOnly self false)
      (Variables|Default|SetbShowMouseCursor false))
    (:then_1
      (if (== (Variables|Default|GetPopup%20Result) "Respawn")
        (Class|UPFPlayerController|Respawn)
        (elif (== (Variables|Default|GetPopup%20Result) "Quit")
          (Class|UPFPlayerController|QuitLevel)
          (else
            (Development|PrintString (Utilities|String|ToString(Text) (Utilities|Text|FormatText "Unknown Popup Result: {PopupResult}" (Variables|Default|GetPopup%20Result))))))))))

(event EventBeginPlay
  (Input|SetInputModeGameOnly self false)
  (if (Pawn|IsLocalPlayerController)
    (bind _returnvalue (UserInterface|CreateWidget "/Game/UnrealPortfolio/UI/BP_UPFHUDWidget.BP_UPFHUDWidget_C" self))
    (bind _output_get (Variables|Default|SetHUDWidget _returnvalue))
    (UserInterface|Viewport|AddtoViewport _output_get 0)))

(event EventTick
  (params (DeltaSeconds :type Float%20%28single-precision%29)))

(event EventOnGameOver
  (if (Pawn|IsLocalPlayerController)
    (CallFunction|ShowGameResultWidget "(TagName=\"GameResult.Fail\")")
    (else
      (Development|PrintString (Utilities|String|ToString(Text) (Utilities|Text|FormatText "Player {PlayerName} Is Dead!!" (Utilities|GetDisplayName self)))))))

(fn ConstructionScript)